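; BP_DeerChar is a player-controlled deer character with movement, steering and camera rotation.
; Forward input moves it along its facing and flags IsSprint near full forward, sideways input yaws the controller, and turn input rotates the spring arm.
; Sprint steps walk speed up by lerp over accumulated time, clearing its timer at MaxTime.
; Nothing shown calls Sprint or reads IsSprint, and StopSprint is empty.
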(event `InputAxis|MoveForward`
  (params (AxisValue :type "Float (single-precision)"))
  (set `self.bIsSprint` (<= (- 1.0 AxisValue) 0.1))
  (`self.AddMovementInput` (`self.GetActorForwardVector`) AxisValue))

(event `InputAxis|MoveRight`
  (params (AxisValue :type "Float (single-precision)"))
  (set `self.AxisValue` AxisValue)
  (`self.AddControllerYawInput` AxisValue))

(event `InputAxis|turn`
  (params (AxisValue :type "Float (single-precision)"))
  (bind _springarm (`self.SpringArm`))
  (`SceneComponent.K2_SetRelativeRotation` _springarm (`KismetMathLibrary.MakeRotator` 0.0 0.0 (+ AxisValue (.yaw (`SpringArmComponent.GetTargetRotation` _springarm)))) false false))

(fn `Sprint`
  (locals (deltaTime :type "Float (double-precision)" :default 0.01) (MaxTime :type "Float (double-precision)" :default 0.5))
  (bind _output_get (set `self.CurrentTime` (+ (`self.CurrentTime`) (`local.deltaTime`))))
  (set `CharacterMovementComponent.MaxWalkSpeed` (`KismetMathLibrary.Lerp` 300.0 600.0 (/ _output_get (`local.MaxTime`))) (`self.CharacterMovement`))
  (if (== (`self.CurrentTime`) (`local.MaxTime`))
    (`KismetSystemLibrary.K2_ClearAndInvalidateTimerHandle` (`self.AccelerateTimer`))
    (set `self.CurrentTime` 0.0)))

(fn `StopSprint`)

(fn `UserConstructionScript`)